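; B_WeaponSounds is an actor that plays weapon fire audio attached to a skeletal mesh.
; Each Fire event reuses the active audio component or spawns a new one with FireTime as its ShotInterval parameter, then sends it a Fire trigger.
; A retriggerable delay, restarted by each shot, repeatedly checks the audio component and destroys the actor once that component is no longer valid.
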(event Custom|Fire
  (Utilities|FlowControl|Sequence
    (:then_0
      (Utilities|IsValid (Variables|Default|GetAudioComponent)
        (:Is%20Valid
          (if (Components|Activation|IsActive (Variables|Default|GetAudioComponent))
            _
            (else
              (bind _returnvalue (Audio|SpawnSoundAttached (Variables|Default|GetFireSound) (Variables|Default|GetSkeletalMeshComponent) "None" "0, 0, 0" "0, 0, 0" "KeepRelativeOffset" false 1.0 1.0 0.0 0 0 :!label _label))
              (bind _output_get (Variables|Default|SetAudioComponent _returnvalue))
              (Audio|Parameter|SetFloatParameter _output_get "ShotInterval" (Variables|Default|GetFireTime) :!class /Script/AudioExtensions.AudioParameterControllerInterface))))
        (:Is%20Not%20Valid
          (goto _label)))
      (Class|AudioParameterControllerInterface|SetTriggerParameter (Variables|Default|GetAudioComponent) "Fire"))
    (:then_1
      (Utilities|FlowControl|RetriggerableDelay 3.0 :!label _label_2)
      (if (Utilities|IsValid (Variables|Default|GetAudioComponent))
        (goto _label_2)
        (else
          (Actor|DestroyActor))))))

(fn ConstructionScript)