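; Base splash-damage area-of-effect actor for projectiles, built on a parent AOE class.
; On BeginPlay it binds the parent's overlap dispatcher to DamageAOE, which sends a damage message using SplashDamage and its own location as knockback epicenter.
; Successful hits report a damage event and notify the instigator of the damage dealt.
; A separate AOEOverlap event launches Characters with a fixed velocity rather than one radiating from the center.
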(event Custom|AOEOverlap
  (params (Actor :type Actor%20Object%20Reference))
  (bind _ascharacter (Utilities|Casting|CastToCharacter Actor))
  (Character|LaunchCharacter _ascharacter "500.000000,500.000000,500.000000" true false))

(event Custom|DamageAOE
  (params (Actor :type Actor%20Object%20Reference))
  (bind _returnvalue (Transformation|GetActorLocation Actor))
  (bind (_wasdamaged _was_damaged_to_death _finaldamage _is_critical_hit) (Class|BPIDamagable|TakeDamage(Message) Actor (Utilities|Struct|MakeS_DamageInfo (Variables|Default|GetSplashDamage) "NewEnumerator3" "NewEnumerator4" false false false true _returnvalue "0.000000,0.000000,0.000000" "None" 1.0) (Game|GetInstigator) (Transformation|GetActorLocation)))
  (if _wasdamaged
    (Class|AISenseDamage|ReportDamageEvent Actor (Game|GetInstigator) _finaldamage (Transformation|GetActorLocation (Game|GetInstigator)) "0, 0, 0" "None")
    (Class|BPIDamagable|DamageDealt(Message) (Game|GetInstigator) _was_damaged_to_death _is_critical_hit _returnvalue _finaldamage)))

(event EventBeginPlay
  (|CallParentFunction)
  (EventDispatchers|AssignOnAOEOverlapActor (delegate Custom|DamageAOE)))

(event Collision|EventActorBeginOverlap
  (params (OtherActor :type Actor%20Object%20Reference))
  (|CallParentFunction OtherActor) ; This node is disabled and will not be called.\nDrag off pins to build functionality.
)

(event EventTick
  (params (DeltaSeconds :type Float%20%28single-precision%29))
  (|CallParentFunction DeltaSeconds) ; This node is disabled and will not be called.\nDrag off pins to build functionality.
)

(fn ConstructionScript
  (|CallParentFunction))