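; Base area-of-effect actor that finds pawns within a radius of its location and reports each one through the OnAOEOverlapActor dispatcher.
; Trigger fires a one-shot sphere overlap, either when called or automatically after a short BeginPlay delay if TriggerOnBeginPlay is set.
; Flags optionally exclude the triggering actor and the Instigator, or draw a debug sphere.
; It applies no effect itself, leaving that to whatever handles the dispatcher.
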(event Custom|Trigger
  (params (TriggerInstigator :type Actor%20Object%20Reference))
  (CallFunction|SpawnAOESphere TriggerInstigator))

(event Custom|SpawnAOESphere
  (params (SpawnInstigator :type Actor%20Object%20Reference))
  (if (Variables|Default|GetDrawDebugSphere)
    (Rendering|Debug|DrawDebugSphere (Transformation|GetActorLocation) (Variables|Default|GetRadius) 12 "(R=1.000000,G=0.000000,B=0.802695,A=1.000000)" 1.0 1.0))
  (bind _outactors (Collision|SphereOverlapActors (Transformation|GetActorLocation) (Variables|Default|GetRadius) (Utilities|Array|MakeArray "ObjectTypeQuery3") 0 (Utilities|Array|MakeArray (select (Variables|Default|GetIgnoreSpawnedFromActor) SpawnInstigator 0) (select (Variables|Default|GetIgnoreInstigator) (Variables|Actor|GetInstigator) 0))))
  (for _array_element _outactors
    (Default|CallOnAOEOverlapActor _array_element)))

(event EventBeginPlay
  (if (Variables|Default|GetTriggerOnBeginPlay)
    (Utilities|FlowControl|Delay 0.1)
    (CallFunction|Trigger)))

(fn ConstructionScript)