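; Base area-of-effect actor for projectile splash, damaging and knocking back what it overlaps.
; On BeginPlay it binds DamageAOE to the overlap dispatcher, sending SplashDamage through a TakeDamageMessage credited to the instigator.
; Successful hits report a damage event, then show a hit marker and damage numbers if the instigator is BP_FirstPersonCharacter.
; AOEOverlap separately launches Characters with a fixed world-space velocity rather than radially from the blast.
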(event Custom|AOEOverlap
  (params (Actor :type Actor%20Object%20Reference))
  (bind _ascharacter (Utilities|Casting|CastToCharacter Actor))
  (Character|LaunchCharacter _ascharacter "500.000000,500.000000,500.000000" true false))

(event Custom|DamageAOE
  (params (Actor :type Actor%20Object%20Reference))
  (bind _returnvalue (Transformation|GetActorLocation Actor))
  (bind (_x _y _z) (Math|Vector|BreakVector _returnvalue))
  (bind (_wasdamaged _was_damaged_to_death) (Class|BPIDamagable|TakeDamage(Message) Actor (Utilities|Struct|MakeS_DamageInfo (Variables|Default|GetSplashDamage) "NewEnumerator3" "NewEnumerator4" false false false true _returnvalue) (Game|GetInstigator)))
  (if _wasdamaged
    (Class|AISenseDamage|ReportDamageEvent Actor (Game|GetInstigator) (Variables|Default|GetSplashDamage) (Transformation|GetActorLocation (Game|GetInstigator)) "0, 0, 0" "None")
    (bind _asbp_first_person_character (Utilities|Casting|CastToBP_FirstPersonCharacter (Game|GetInstigator)))
    (Default|PlayHitMarker (Variables|/Game/FirstPerson/Blueprints/BP_FirstPersonCharacter.BP_FirstPersonCharacter_C|GetPlayerHUDRef _asbp_first_person_character) _was_damaged_to_death)
    (Default|SpawnDamageNumbers (Variables|Default|GetBPC_DamageNumbers) (Utilities|Array|MakeArray (Math|Vector4|MakeVector4 _x _y _z (Variables|Default|GetSplashDamage))))))

(event EventBeginPlay
  (|CallParentFunction)
  (EventDispatchers|AssignOnAOEOverlapActor (delegate Custom|DamageAOE)))

(event Collision|EventActorBeginOverlap
  (params (OtherActor :type Actor%20Object%20Reference))
  (|CallParentFunction OtherActor) ; This node is disabled and will not be called.\nDrag off pins to build functionality.
)

(event EventTick
  (params (DeltaSeconds :type Float%20%28single-precision%29))
  (|CallParentFunction DeltaSeconds) ; This node is disabled and will not be called.\nDrag off pins to build functionality.
)

(fn ConstructionScript
  (|CallParentFunction))