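; Base weapon pickup that attaches its WeaponComponent to the player when set in use and responds to its delegates.
; Equip and stow toggle the HUD ammo display and scope reticle.
; Hitscan fire applies damage and drives lazily spawned, reused actors for weapon FX, decals, impacts and sound.
; Projectile fire spawns an aimed projectile whose impact deals direct damage plus optional reduced AOE splash, with hit markers and damage numbers.
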(event OnStowDelegate(WeaponComponent)
  (params (Character :type Octahedron%20Character%20Object%20Reference) (Weapon :type TP%20Weapon%20Component%20Object%20Reference))
  (bind _asbp_first_person_character (Utilities|Casting|CastToBP_FirstPersonCharacter Character))
  (bind _output_get (Variables|Default|SetCharacter _asbp_first_person_character))
  (Default|UpdateCurrentAmmo (Variables|/Game/FirstPerson/Blueprints/BP_FirstPersonCharacter.BP_FirstPersonCharacter_C|GetPlayerHUDRef _output_get) (Variables|/Script/Octahedron.TP_WeaponComponent|GetCurrentMagazineCount Weapon))
  (bind _returnvalue (Class|OctahedronCharacter|GetRemainingAmmo _output_get (Variables|/Script/Octahedron.TP_WeaponComponent|GetAmmoType Weapon)))
  (Default|UpdateRemainingAmmo (Variables|/Game/FirstPerson/Blueprints/BP_FirstPersonCharacter.BP_FirstPersonCharacter_C|GetPlayerHUDRef _output_get) _returnvalue)
  (Widget|SetRenderOpacity (Variables|/Game/UI/Hud/Widgets/W_PlayerHUD.W_PlayerHUD_C|GetCurrentAmmo (Variables|/Game/FirstPerson/Blueprints/BP_FirstPersonCharacter.BP_FirstPersonCharacter_C|GetPlayerHUDRef _output_get)) 0.0)
  (Widget|SetRenderOpacity (Variables|/Game/UI/Hud/Widgets/W_PlayerHUD.W_PlayerHUD_C|GetRemainingAmmo (Variables|/Game/FirstPerson/Blueprints/BP_FirstPersonCharacter.BP_FirstPersonCharacter_C|GetPlayerHUDRef _output_get)) 0.0)
  (Widget|SetRenderOpacity (Variables|/Game/UI/Hud/Widgets/W_PlayerHUD.W_PlayerHUD_C|GetAmmoSlash (Variables|/Game/FirstPerson/Blueprints/BP_FirstPersonCharacter.BP_FirstPersonCharacter_C|GetPlayerHUDRef _output_get)) 0.0)
  (bind _scopesightmesh (Variables|/Script/Octahedron.TP_WeaponComponent|GetScopeSightMesh Weapon)
    (:then
      (if (Variables|/Script/Octahedron.SightMeshComponent|GetIsReticleExist _scopesightmesh)
        (bind _createdreticlewidget (Variables|Default|GetCreatedReticleWidget)
          (:then
            (Widget|RemovefromParent _createdreticlewidget))
          (:else)))
      (CallFunction|SetinUse false))
    (:else)))

(event OnWeaponHitScanFireDelegate(WeaponComponent)
  (params (HitResults :type Array%20of%20Hit%20Result%20Structures))
  (Default|UpdateCurrentAmmo (Variables|/Game/FirstPerson/Blueprints/BP_FirstPersonCharacter.BP_FirstPersonCharacter_C|GetPlayerHUDRef (Variables|Default|GetCharacter)) (Variables|/Script/Octahedron.TP_WeaponComponent|GetCurrentMagazineCount (Variables|Default|GetWeaponComponent)))
  (bind (_isdamagedealt _isdamagedtodeath) (CallFunction|DeployHitScanFiredFX HitResults))
  (if _isdamagedealt
    (Default|PlayHitMarker (Variables|/Game/FirstPerson/Blueprints/BP_FirstPersonCharacter.BP_FirstPersonCharacter_C|GetPlayerHUDRef (Variables|Default|GetCharacter)) _isdamagedtodeath)))

(event OnWeaponProjectileFireDelegate(WeaponComponent)
  (params (HitResult :type Hit%20Result%20Structure))
  (bind (_bblockinghit _binitialoverlap _time _distance _location _impactpoint _normal _impactnormal _physmat _hitactor _hitcomponent _hitbonename _bonename _hititem _elementindex _faceindex _tracestart _traceend) (Collision|BreakHitResult HitResult))
  (bind _muzzlesocket (Variables|Default|GetMuzzleSocket))
  (bind _character (Variables|Default|GetCharacter))
  (bind _weaponcomponent (Variables|Default|GetWeaponComponent))
  (bind _returnvalue (Transformation|GetSocketLocation _weaponcomponent _muzzlesocket))
  (Default|UpdateCurrentAmmo (Variables|/Game/FirstPerson/Blueprints/BP_FirstPersonCharacter.BP_FirstPersonCharacter_C|GetPlayerHUDRef (Variables|Default|GetCharacter)) (Variables|/Script/Octahedron.TP_WeaponComponent|GetCurrentMagazineCount (Variables|Default|GetWeaponComponent)))
  (CallFunction|DeployProjectileFiredFX HitResult)
  (bind _returnvalue_2 (Game|SpawnActorfromClass (Variables|Default|GetCustomProjectile) (Math|Transform|MakeTransform _returnvalue (Math|Rotator|FindLookatRotation _returnvalue (select _bblockinghit _location _traceend)) "1.000000,1.000000,1.000000") "Undefined" "MultiplyWithRoot" _character 1e+03 0.0 false 2e+03 false 0 _character))
  (Collision|IgnoreActorwhenMoving (Variables|/Script/Engine.Character|GetCapsuleComponent (Variables|Default|GetCharacter)) _returnvalue_2 true)
  (EventDispatchers|BindEventtoOnProjectileImpactDelegate _returnvalue_2 (delegate Custom|ProjectileImpact)))

(event OnEquipDelegate(WeaponComponent)
  (params (Character :type Octahedron%20Character%20Object%20Reference) (Weapon :type TP%20Weapon%20Component%20Object%20Reference))
  (bind _asbp_first_person_character (Utilities|Casting|CastToBP_FirstPersonCharacter Character))
  (bind _output_get (Variables|Default|SetCharacter _asbp_first_person_character))
  (Default|UpdateCurrentAmmo (Variables|/Game/FirstPerson/Blueprints/BP_FirstPersonCharacter.BP_FirstPersonCharacter_C|GetPlayerHUDRef _output_get) (Variables|/Script/Octahedron.TP_WeaponComponent|GetCurrentMagazineCount Weapon))
  (bind _returnvalue (Class|OctahedronCharacter|GetRemainingAmmo _output_get (Variables|/Script/Octahedron.TP_WeaponComponent|GetAmmoType Weapon)))
  (Default|UpdateRemainingAmmo (Variables|/Game/FirstPerson/Blueprints/BP_FirstPersonCharacter.BP_FirstPersonCharacter_C|GetPlayerHUDRef _output_get) _returnvalue)
  (Widget|SetRenderOpacity (Variables|/Game/UI/Hud/Widgets/W_PlayerHUD.W_PlayerHUD_C|GetCurrentAmmo (Variables|/Game/FirstPerson/Blueprints/BP_FirstPersonCharacter.BP_FirstPersonCharacter_C|GetPlayerHUDRef _output_get)) 1.0)
  (Widget|SetRenderOpacity (Variables|/Game/UI/Hud/Widgets/W_PlayerHUD.W_PlayerHUD_C|GetRemainingAmmo (Variables|/Game/FirstPerson/Blueprints/BP_FirstPersonCharacter.BP_FirstPersonCharacter_C|GetPlayerHUDRef _output_get)) 1.0)
  (Widget|SetRenderOpacity (Variables|/Game/UI/Hud/Widgets/W_PlayerHUD.W_PlayerHUD_C|GetAmmoSlash (Variables|/Game/FirstPerson/Blueprints/BP_FirstPersonCharacter.BP_FirstPersonCharacter_C|GetPlayerHUDRef _output_get)) 1.0)
  (bind _scopesightmesh (Variables|/Script/Octahedron.TP_WeaponComponent|GetScopeSightMesh Weapon)
    (:then
      (if (Variables|/Script/Octahedron.SightMeshComponent|GetIsReticleExist _scopesightmesh)
        (bind _returnvalue_2 (UserInterface|CreateWidget (Variables|/Script/Octahedron.TP_WeaponComponent|GetScopeReticleWidget Weapon) (Pawn|GetLocalViewingPlayerController _output_get)))
        (bind _output_get_2 (Variables|Default|SetCreatedReticleWidget _returnvalue_2))
        (UserInterface|Viewport|AddtoPlayerScreen _output_get_2)))
    (:else)))

(event Custom|ProjectileImpact
  (params (OtherActor :type Actor%20Object%20Reference) (Hit :type Hit%20Result%20Structure))
  (bind (_bblockinghit _binitialoverlap _time _distance _location _impactpoint _normal _impactnormal _physmat _hitactor _hitcomponent _hitbonename) (Collision|BreakHitResult Hit))
  (bind _aoeclass (Variables|Default|GetAOEClass))
  (if (Utilities|IsValidClass _aoeclass)
    (bind _returnvalue (Game|SpawnActorfromClass _aoeclass (Math|Transform|MakeTransform _location "0, 0, 0" "1.000000,1.000000,1.000000") "Undefined" "MultiplyWithRoot" 0 false false false true (Variables|Default|GetCharacter)))
    (bind _asbp_aoe_projectile_splash_base (Utilities|Casting|CastToBP_AOE_ProjectileSplash_Base _returnvalue))
    (Variables|/Game/AOE/Splash/BP_AOE_ProjectileSplash_Base.BP_AOE_ProjectileSplash_Base_C|SetSplashDamage _asbp_aoe_projectile_splash_base (* (Variables|/Script/Octahedron.TP_WeaponComponent|GetDamage (Variables|Default|GetWeaponComponent)) 0.65))
    (Default|Trigger _asbp_aoe_projectile_splash_base OtherActor))
  (bind (_wasdamaged _was_damaged_to_death _finaldamage _is_critical_hit) (Class|BPIDamagable|TakeDamage(Message) OtherActor (Utilities|Struct|MakeS_DamageInfo (Variables|/Script/Octahedron.TP_WeaponComponent|GetDamage (Variables|Default|GetWeaponComponent)) "NewEnumerator2" "NewEnumerator4" false false false true _location _normal _hitbonename 1.0) (Variables|Default|GetCharacter) _location))
  (if _wasdamaged
    (Class|AISenseDamage|ReportDamageEvent OtherActor (Variables|Default|GetCharacter) _finaldamage (Transformation|GetActorLocation (Variables|Default|GetCharacter)) "0, 0, 0" "None")
    (Default|PlayHitMarker (Variables|/Game/FirstPerson/Blueprints/BP_FirstPersonCharacter.BP_FirstPersonCharacter_C|GetPlayerHUDRef (Variables|Default|GetCharacter)) _was_damaged_to_death)
    (Default|SpawnDamageNumbers (Variables|Default|GetBPC_DamageNumbers) _location _finaldamage _is_critical_hit)))

(event Collision|EventActorBeginOverlap
  (params (OtherActor :type Actor%20Object%20Reference)))

(event EventTick
  (params (DeltaSeconds :type Float%20%28single-precision%29)))

(event EventSetinUse
  (params (InUse :type Boolean))
  (|CallParentFunction InUse)
  (if InUse
    (bind _asoctahedron_character (Utilities|Casting|CastToOctahedronCharacter (Game|GetPlayerCharacter 0)))
    (Class|TPWeaponComponent|AttachWeapon (Variables|Default|GetWeaponComponent) _asoctahedron_character)))

(fn ConstructionScript)

(fn AddFakeProjectileData
  (params (Number%20Of%20Fake%20Projectiles :type Integer) (Cone%20Half%20Angle%20In%20Degrees :type Float%20%28double-precision%29))
  (bind _weaponcomponent (Variables|Default|GetWeaponComponent))
  (bind _returnvalue (Transformation|GetSocketTransform _weaponcomponent "Muzzle" "RTS_World"))
  (bind _location (Math|Transform|BreakTransform _returnvalue))
  (for _index (range 1 (Math|Integer|Max(Integer) Number%20Of%20Fake%20Projectiles))
    (bind (_outhit _returnvalue_2) (Collision|LineTraceByChannel _location (+ (* (Math|Random|RandomUnitVectorinConeinDegrees (Math|Vector|Normalize (- (Utilities|Array|Get(acopy) (Variables|Default|GetImpact%20Positions)) _location)) Cone%20Half%20Angle%20In%20Degrees) 1e+06) _location) "TraceTypeQuery1" false 0 "None"))
    ;[1 1 1] Append Fake projectile hits to the impact arrays
    (if _returnvalue_2
      (Utilities|Array|Add (Variables|Default|GetImpact%20Positions) (.Location (Collision|BreakHitResult _outhit)))
      (Utilities|Array|Add (Variables|Default|GetImpact%20Normals) (.Normal (Collision|BreakHitResult _outhit))))))

(fn DeployHitScanFiredFX
  (params (HitResults :type Array%20of%20Hit%20Result%20Structures))
  (bind _weaponcomponent (Variables|Default|GetWeaponComponent))
  (bind _character (Variables|Default|GetCharacter))
  (Utilities|FlowControl|Sequence
    (:then_0
      ;[1 1 1] Save hit result Info and apply damage if applicable
      (Utilities|Array|Clear (Variables|Default|GetImpact%20Positions))
      (Utilities|Array|Clear (Variables|Default|GetImpact%20Normals))
      (Utilities|Array|Clear (Variables|Default|GetImpactSurfaceTypes))
      (Utilities|Array|Clear (Variables|Default|GetTracerPositions))
      (for _array_element HitResults
        (if (.bBlockingHit (Collision|BreakHitResult _array_element))
          (Utilities|Array|Add (Variables|Default|GetTracerPositions) (.Location (Collision|BreakHitResult _array_element)))
          (Utilities|Array|Add (Variables|Default|GetImpact%20Positions) (.Location (Collision|BreakHitResult _array_element)))
          (Utilities|Array|Add (Variables|Default|GetImpact%20Normals) (.Normal (Collision|BreakHitResult _array_element)))
          (Utilities|Array|Add (Variables|Default|GetImpactSurfaceTypes) (Variables|/Script/PhysicsCore.PhysicalMaterial|GetSurfaceType (.PhysMat (Collision|BreakHitResult _array_element))))
          (bind (_wasdamaged _was_damaged_to_death _finaldamage _is_critical_hit) (Class|BPIDamagable|TakeDamage(Message) (.HitActor (Collision|BreakHitResult _array_element)) (Utilities|Struct|MakeS_DamageInfo (Variables|/Script/Octahedron.TP_WeaponComponent|GetDamage (Variables|Default|GetWeaponComponent)) "NewEnumerator2" "NewEnumerator1" false false false false (.Location (Collision|BreakHitResult _array_element)) (.Normal (Collision|BreakHitResult _array_element)) (.HitBoneName (Collision|BreakHitResult _array_element)) 1.0) (Variables|Default|GetCharacter) "0, 0, 0"))
          (if _wasdamaged
            (Default|SpawnDamageNumbers (Variables|Default|GetBPC_DamageNumbers) (.Location (Collision|BreakHitResult _array_element)) _finaldamage _is_critical_hit)
            (Class|AISenseDamage|ReportDamageEvent (.HitActor (Collision|BreakHitResult _array_element)) _character _finaldamage (Transformation|GetActorLocation _character) "0, 0, 0" "None")
            (LocalVariables|SetWasDamaged true)
            (LocalVariables|SetWasDamagedToDeath _was_damaged_to_death))
          (else
            (Utilities|Array|Add (Variables|Default|GetTracerPositions) (.TraceEnd (Collision|BreakHitResult _array_element))))))
      (Variables|Default|SetMuzzle%20Position (Transformation|GetSocketLocation (Variables|Default|GetWeaponComponent) (Variables|Default|GetMuzzleSocket))))
    (:then_1
      ;[1 1 1] Muzzle Flash, Tracer, and Shell Eject
      (Utilities|IsValid (Variables|Niagara|GetBP_WeaponFX)
        (:Is%20Valid
          _)
        (:Is%20Not%20Valid
          (bind _returnvalue (Game|SpawnActorfromClass "/Game/Weapons/Effects/BP_WeaponFX.BP_WeaponFX_C" (Math|Transform|MakeTransform "0, 0, 0") "Undefined" "MultiplyWithRoot" 0 (Variables|Default|GetWeaponComponent) (Variables|Niagara|GetMuzzle%20Flash%20FX) (Variables|Niagara|GetTracer%20FX) (Variables|Niagara|GetShell%20Eject%20Mesh) (Variables|Default|GetMuzzleSocket) (Variables|Default|GetShellEjectSocket) 0))
          (bind _output_get (Variables|Niagara|SetBP_WeaponFX _returnvalue))
          (Transformation|AttachComponentToComponent _output_get (Variables|Default|GetWeaponComponent) "None" "KeepRelative" "KeepRelative" "KeepRelative" true)))
      (Default|WeaponFired (Variables|Niagara|GetBP_WeaponFX) (Variables|Default|GetTracerPositions)))
    (:then_2
      ;[1 1 1] Bullet Decals
      (Utilities|IsValid (Variables|Niagara|GetBP_WeaponDecalsFX)
        (:Is%20Valid
          _)
        (:Is%20Not%20Valid
          (bind _returnvalue_2 (Game|SpawnActorfromClass "/Game/Weapons/Effects/BP_WeaponDecals.BP_WeaponDecals_C" (Math|Transform|MakeTransform "0, 0, 0") "Undefined" "MultiplyWithRoot" 0 0))
          (bind _output_get_2 (Variables|Niagara|SetBP_WeaponDecalsFX _returnvalue_2))
          (Transformation|AttachComponentToComponent _output_get_2 (Variables|Default|GetWeaponComponent) "None" "KeepRelative" "KeepRelative" "KeepRelative" true)))
      (Default|WeaponFired (Variables|Niagara|GetBP_WeaponDecalsFX) (Variables|Default|GetImpact%20Positions) (Variables|Default|GetImpact%20Normals) (Variables|Default|GetImpactSurfaceTypes) (Variables|Default|GetMuzzle%20Position)))
    (:then_3
      ;[1 1 1] Weapon Impact
      (if (Utilities|Array|IsNotEmpty (Variables|Default|GetImpact%20Positions))
        (Utilities|IsValid (Variables|Niagara|GetBP_WeaponImpactsFX)
          (:Is%20Valid
            _)
          (:Is%20Not%20Valid
            (bind _returnvalue_3 (Game|SpawnActorfromClass "/Game/Weapons/Effects/BP_WeaponImpacts.BP_WeaponImpacts_C" (Math|Transform|MakeTransform "0, 0, 0") "Undefined" "MultiplyWithRoot" 0 0))
            (bind _output_get_3 (Variables|Niagara|SetBP_WeaponImpactsFX _returnvalue_3))
            (Transformation|AttachComponentToComponent _output_get_3 (Variables|Default|GetWeaponComponent) "None" "KeepRelative" "KeepRelative" "KeepRelative" true)))
        (Default|WeaponFired (Variables|Niagara|GetBP_WeaponImpactsFX) (Variables|Default|GetImpact%20Positions) (Variables|Default|GetImpact%20Normals) (Variables|Default|GetImpactSurfaceTypes) (Variables|Default|GetMuzzle%20Position))))
    (:then_4
      ;[1 1 1] Weapon Fire Sounds
      (Utilities|IsValid (Variables|Default|GetWeaponSounds)
        (:Is%20Valid
          _)
        (:Is%20Not%20Valid
          (bind _returnvalue_4 (Game|SpawnActorfromClass "/Game/Effects/Blueprints/B_WeaponSounds.B_WeaponSounds_C" (Math|Transform|MakeTransform "0, 0, 0") "Undefined" "MultiplyWithRoot" 0 (Variables|Default|GetWeaponComponent) (* (Variables|/Script/Octahedron.TP_WeaponComponent|GetFireDelay _weaponcomponent) (Variables|/Script/Octahedron.TP_WeaponComponent|GetFireSoundDelayScale _weaponcomponent)) (Variables|/Script/Octahedron.TP_WeaponComponent|GetFireSound (Variables|Default|GetWeaponComponent)) 0))
          (bind _output_get_4 (Variables|Default|SetWeaponSounds _returnvalue_4))
          (Transformation|AttachComponentToComponent _output_get_4 (Variables|Default|GetWeaponComponent) "None" "KeepRelative" "KeepRelative" "KeepRelative" true)))
      (Default|Fire (Variables|Default|GetWeaponSounds)))
    (:then_5
      (return (LocalVariables|GetWasDamaged) (LocalVariables|GetWasDamagedToDeath)))))

(fn DeployProjectileFiredFX
  (params (HitResult :type Hit%20Result%20Structure))
  (bind _weaponcomponent (Variables|Default|GetWeaponComponent))
  (bind _muzzlesocket (Variables|Default|GetMuzzleSocket))
  (Audio|PlaySoundatLocation (Variables|/Game/Weapons/Default/Parent_BP/BP_WeaponComponent_Base.BP_WeaponComponent_Base_C|GetProjectileFireSFX (Variables|Default|GetWeaponComponent)) (Transformation|GetSocketLocation (Variables|Default|GetWeaponComponent) (Variables|Default|GetMuzzleSocket)) "0, 0, 0" 1.0 1.0 0.0 0 0 0 0)
  (Effects|SpawnEmitteratLocation (Variables|/Game/Weapons/Default/Parent_BP/BP_WeaponComponent_Base.BP_WeaponComponent_Base_C|GetProjectileFireEmitter (Variables|Default|GetWeaponComponent)) (Transformation|GetSocketLocation _weaponcomponent _muzzlesocket) (Transformation|GetSocketRotation _weaponcomponent _muzzlesocket)))