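; Weapon effects actor that plays muzzle flash, shell eject and tracer Niagara systems when WeaponFired supplies impact positions.
; Each system spawns attached at a weapon mesh socket offset, is reused while active, and fires per shot by flipping a User.Trigger bool.
; Impact positions aim the muzzle flash and feed the tracer's array parameter.
; A retriggerable delay loop destroys the actor once all three auto-destroying systems are gone.
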(event Custom|WeaponFired
  (params (ImpactPositions :type Array%20of%20Vectors))
  (Variables|Default|SetImpact%20Positions ImpactPositions)
  (Utilities|FlowControl|Sequence
    (:then_0
      (Utilities|IsValid (Variables|Default|GetNS_MuzzleFlash)
        (:Is%20Valid
          (if (Components|Activation|IsActive (Variables|Default|GetNS_MuzzleFlash))
            _
            (else
              (bind _returnvalue (Niagara|SpawnSystemAttached (Variables|Default|GetMuzzleFlashFX) (Variables|Default|GetDefaultSceneRoot) "None" (.location (Transformation|GetSocketTransform (Variables|Default|GetWeaponMesh) (Variables|Default|GetMuzzleSocket) "RTS_Component")) "0.000000,0.000000,0.000000" "KeepRelativeOffset" true :!label _label))
              (Variables|Default|SetNS_MuzzleFlash _returnvalue)
              (Variables|Default|SetMuzzleFlashTrigger false))))
        (:Is%20Not%20Valid
          (goto _label)))
      (Variables|Default|SetMuzzleFlashTrigger (not (Variables|Default|GetMuzzleFlashTrigger)))
      (Niagara|SetNiagaraVariable(Vector3) (Variables|Default|GetNS_MuzzleFlash) "User.Direction" (Math|Vector|Normalize (- (Utilities|Array|Get(acopy) (Variables|Default|GetImpact%20Positions)) (.Location (Math|Transform|BreakTransform (Transformation|GetSocketTransform (Variables|Default|GetWeaponMesh) (Variables|Default|GetMuzzleSocket) "RTS_World"))))))
      (Class|NiagaraComponent|SetVariableBool (Variables|Default|GetNS_MuzzleFlash) "User.Trigger" (Variables|Default|GetMuzzleFlashTrigger)))
    (:then_1
      (Utilities|IsValid (Variables|Default|GetNS_ShellEject)
        (:Is%20Valid
          (if (Components|Activation|IsActive (Variables|Default|GetNS_ShellEject))
            _
            (else
              (bind _returnvalue_2 (Niagara|SpawnSystemAttached (Variables|Default|GetShellEjectFX) (Variables|Default|GetDefaultSceneRoot) "None" (.location (Transformation|GetSocketTransform (Variables|Default|GetWeaponMesh) (Variables|Default|GetShellEjectSocket) "RTS_Component")) "0.000000,90.000000,0.000000" "KeepRelativeOffset" true :!label _label_2))
              (Variables|Default|SetNS_ShellEject _returnvalue_2)
              (Class|NiagaraComponent|SetVariableStaticMesh (Variables|Default|GetNS_ShellEject) "User.ShellEjectStaticMesh" (Variables|Default|GetShellEjectMesh))
              (Variables|Default|SetShellEjectTrigger false))))
        (:Is%20Not%20Valid
          (goto _label_2)))
      (Variables|Default|SetShellEjectTrigger (not (Variables|Default|GetShellEjectTrigger)))
      (Class|NiagaraComponent|SetVariableBool (Variables|Default|GetNS_ShellEject) "User.Trigger" (Variables|Default|GetShellEjectTrigger)))
    (:then_2
      (Utilities|IsValid (Variables|Default|GetNS_Tracer)
        (:Is%20Valid
          (if (Components|Activation|IsActive (Variables|Default|GetNS_Tracer))
            _
            (else
              (bind _returnvalue_3 (Niagara|SpawnSystemAttached (Variables|Default|GetTracerFX) (Variables|Default|GetDefaultSceneRoot) "None" (.location (Transformation|GetSocketTransform (Variables|Default|GetWeaponMesh) (Variables|Default|GetMuzzleSocket) "RTS_Component")) "0.000000,90.000000,0.000000" "KeepRelativeOffset" true :!label _label_3))
              (Variables|Default|SetNS_Tracer _returnvalue_3)
              (Variables|Default|SetTracerTrigger false))))
        (:Is%20Not%20Valid
          (goto _label_3)))
      (Variables|Default|SetTracerTrigger (not (Variables|Default|GetTracerTrigger)))
      (Class|NiagaraComponent|SetVariableBool (Variables|Default|GetNS_Tracer) "User.Trigger" (Variables|Default|GetTracerTrigger))
      (Class|NiagaraDataInterfaceArrayFunctionLibrary|SetNiagaraArrayVector (Variables|Default|GetNS_Tracer) "User.ImpactPositions" (Variables|Default|GetImpact%20Positions)))
    (:then_3
      (Utilities|FlowControl|RetriggerableDelay 0.2 :!label _label_4)
      (if (Math|Boolean|ORBoolean (Utilities|IsValid (Variables|Default|GetNS_MuzzleFlash)) (Utilities|IsValid (Variables|Default|GetNS_ShellEject)) (Utilities|IsValid (Variables|Default|GetNS_Tracer)))
        (goto _label_4)
        (else
          (Actor|DestroyActor))))))

(fn ConstructionScript)