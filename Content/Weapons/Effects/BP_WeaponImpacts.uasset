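; Weapon impact effects actor that turns each WeaponFired event's hits into surface-specific Niagara effects.
; Hits are split by surface type: concrete and glass feed arrays into reused systems, while body and default hits spawn individual sparks.
; Body hits also feed damage numbers, using a hardcoded damage value, for the locally controlled player.
; A retriggerable delay destroys the actor once its tracked systems are gone.
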(event Custom|WeaponFired
  (params (ImpactPositions :type Array%20of%20Vectors) (ImpactNormals :type Array%20of%20Vectors) (ImpactSurfaces :type Array%20of%20EPhysicalSurface%20Enums :default "SurfaceType_Default") (MuzzlePosition :type Vector))
  (Variables|Default|SetImpact%20Positions ImpactPositions)
  (Variables|Default|SetImpact%20Normals ImpactNormals)
  (Variables|Default|SetImpact%20Surfaces ImpactSurfaces)
  (Variables|Default|SetMuzzle%20Position MuzzlePosition)
  (CallFunction|SplitArraybySurfaces)
  (Utilities|FlowControl|Sequence
    (:then_0
      (if (Utilities|Array|IsNotEmpty (Variables|Default|GetConcreteImpacts))
        (Utilities|IsValid (Variables|Default|GetNS_Concrete)
          (:Is%20Valid
            (if (Components|Activation|IsActive (Variables|Default|GetNS_Concrete))
              (Transformation|SetWorldLocation (Variables|Default|GetNS_Concrete) (Utilities|Array|Get(acopy) (Variables|Default|GetConcreteImpacts)) false false)
              (else
                (bind _returnvalue (Niagara|SpawnSystematLocation "/Game/Effects/Particles/Impacts/NS_ImpactConcrete.NS_ImpactConcrete" (Utilities|Array|Get(acopy) (Variables|Default|GetConcreteImpacts)) :!label _label))
                (Variables|Default|SetNS_Concrete _returnvalue))))
          (:Is%20Not%20Valid
            (goto _label)))
        (Class|NiagaraDataInterfaceArrayFunctionLibrary|SetNiagaraArrayPosition (Variables|Default|GetNS_Concrete) "User.ImpactPositions" (Variables|Default|GetConcreteImpacts))
        (Class|NiagaraDataInterfaceArrayFunctionLibrary|SetNiagaraArrayVector (Variables|Default|GetNS_Concrete) "User.ImpactNormals" (Variables|Default|GetConcreteNormals))
        (Class|NiagaraComponent|SetVariableInt (Variables|Default|GetNS_Concrete) "User.NumberOfHits" (Utilities|Array|Length (Variables|Default|GetConcreteImpacts)))
        (Class|NiagaraComponent|SetVariablePosition (Variables|Default|GetNS_Concrete) "User.MuzzlePosition" (Variables|Default|GetMuzzle%20Position))
        (Components|Activation|Activate (Variables|Default|GetNS_Concrete) false)))
    (:then_1
      (if (Utilities|Array|IsNotEmpty (Variables|Default|GetGlassImpacts))
        (Utilities|IsValid (Variables|Default|GetNS_Glass)
          (:Is%20Valid
            (if (Components|Activation|IsActive (Variables|Default|GetNS_Glass))
              (Transformation|SetWorldLocation (Variables|Default|GetNS_Glass) (Utilities|Array|Get(acopy) (Variables|Default|GetGlassImpacts)) false false)
              (else
                (bind _returnvalue_2 (Niagara|SpawnSystematLocation "/Game/Effects/Particles/Impacts/NS_ImpactGlass.NS_ImpactGlass" (Utilities|Array|Get(acopy) (Variables|Default|GetGlassImpacts)) :!label _label_2))
                (Variables|Default|SetNS_Glass _returnvalue_2))))
          (:Is%20Not%20Valid
            (goto _label_2)))
        (Class|NiagaraDataInterfaceArrayFunctionLibrary|SetNiagaraArrayPosition (Variables|Default|GetNS_Glass) "User.ImpactPositions" (Variables|Default|GetGlassImpacts))
        (Class|NiagaraDataInterfaceArrayFunctionLibrary|SetNiagaraArrayVector (Variables|Default|GetNS_Glass) "User.ImpactNormals" (Variables|Default|GetGlassNormals))
        (Class|NiagaraComponent|SetVariableInt (Variables|Default|GetNS_Glass) "User.NumberOfHits" (Utilities|Array|Length (Variables|Default|GetGlassImpacts)))
        (Class|NiagaraComponent|SetVariablePosition (Variables|Default|GetNS_Glass) "User.MuzzlePosition" (Variables|Default|GetMuzzle%20Position))
        (Components|Activation|Activate (Variables|Default|GetNS_Glass) false)))
    (:then_2
      (if (Utilities|Array|IsNotEmpty (Variables|Default|GetBodyImpacts))
        (for (_array_element _array_index) (Variables|Default|GetBodyImpacts)
          (Utilities|Array|SetArrayElem (Variables|Default|GetDamageInfo) _array_index (Math|Vector4|MakeVector4 (.X (Math|Vector|BreakVector _array_element)) (.Y (Math|Vector|BreakVector _array_element)) (.Z (Math|Vector|BreakVector _array_element)) 12.0) true)
          (Niagara|SpawnSystematLocation "/Game/Effects/Particles/Impacts/NS_ImactSparksCharacter.NS_ImactSparksCharacter" _array_element (Math|Conversions|RotationFromXVector (Utilities|Array|Get(acopy) (Variables|Default|GetBodyNormals) _array_index))))
        ;[1 1 1] Damage Numbers
        (if (Pawn|IsLocallyControlled (Variables|Default|GetOwningPlayer))
          (Utilities|IsValid (Variables|Default|GetNS_DamageNumbers)
            (:Is%20Valid
              (if (Components|Activation|IsActive (Variables|Default|GetNS_DamageNumbers))
                (Transformation|SetWorldLocation (Variables|Default|GetNS_DamageNumbers) (Utilities|Array|Get(acopy) (Variables|Default|GetBodyImpacts)) false false)
                (else
                  (bind _returnvalue_3 (Niagara|SpawnSystematLocation "/Game/Effects/Particles/Impacts/NS_DamageNumbers.NS_DamageNumbers" (Utilities|Array|Get(acopy) (Variables|Default|GetBodyImpacts)) :!label _label_3))
                  (Variables|Default|SetNS_DamageNumbers _returnvalue_3))))
            (:Is%20Not%20Valid
              (goto _label_3)))
          (Class|NiagaraDataInterfaceArrayFunctionLibrary|SetNiagaraArrayVector4 (Variables|Default|GetNS_DamageNumbers) "User.DamageInfo" (Variables|Default|GetDamageInfo))
          (Class|NiagaraComponent|SetVariableBool (Variables|Default|GetNS_DamageNumbers) "None" false))))
    (:then_3
      (if (Utilities|Array|IsNotEmpty (Variables|Default|GetDefaultImpacts))
        (for (_array_element_2 _array_index_2) (Variables|Default|GetDefaultImpacts)
          (Niagara|SpawnSystematLocation "/Game/Effects/Particles/Impacts/NS_ImactSparksCharacter.NS_ImactSparksCharacter" _array_element_2 (Math|Conversions|RotationFromXVector (Utilities|Array|Get(acopy) (Variables|Default|GetDefaultNormals) _array_index_2))))))
    (:then_4
      (Utilities|Array|Clear (Variables|Default|GetBodyImpacts))
      (Utilities|Array|Clear (Variables|Default|GetBodyNormals))
      (Utilities|Array|Clear (Variables|Default|GetConcreteImpacts))
      (Utilities|Array|Clear (Variables|Default|GetConcreteNormals))
      (Utilities|Array|Clear (Variables|Default|GetGlassImpacts))
      (Utilities|Array|Clear (Variables|Default|GetGlassNormals))
      (Utilities|Array|Clear (Variables|Default|GetDefaultImpacts))
      (Utilities|Array|Clear (Variables|Default|GetDefaultNormals))
      (Utilities|Array|Clear (Variables|Default|GetDamageInfo)))
    (:then_5
      (Utilities|FlowControl|RetriggerableDelay 3.0 :!label _label_4)
      (if (Math|Boolean|ORBoolean (Utilities|IsValid (Variables|Default|GetNS_Concrete)) (Utilities|IsValid (Variables|Default|GetNS_Glass)) (Utilities|IsValid (Variables|Default|GetNS_DamageNumbers)))
        (goto _label_4)
        (else
          (Actor|DestroyActor))))))

(fn ConstructionScript)

(fn SplitArraybySurfaces
  (for (_array_element _array_index) (Variables|Default|GetImpact%20Surfaces)
    (if (Utilities|Enum|Equal(Enum) _array_element "SurfaceType_Default")
      (Utilities|Array|Add (Variables|Default|GetDefaultImpacts) (Utilities|Array|Get(acopy) (Variables|Default|GetImpact%20Positions) _array_index))
      (Utilities|Array|Add (Variables|Default|GetDefaultNormals) (Utilities|Array|Get(acopy) (Variables|Default|GetImpact%20Normals) _array_index))
      (elif (Utilities|Enum|Equal(Enum) _array_element "SurfaceType1")
        (Utilities|Array|Add (Variables|Default|GetBodyImpacts) (Utilities|Array|Get(acopy) (Variables|Default|GetImpact%20Positions) _array_index))
        (Utilities|Array|Add (Variables|Default|GetBodyNormals) (Utilities|Array|Get(acopy) (Variables|Default|GetImpact%20Normals) _array_index))
        (elif (Utilities|Enum|Equal(Enum) _array_element "SurfaceType2")
          (Utilities|Array|Add (Variables|Default|GetConcreteImpacts) (Utilities|Array|Get(acopy) (Variables|Default|GetImpact%20Positions) _array_index))
          (Utilities|Array|Add (Variables|Default|GetConcreteNormals) (Utilities|Array|Get(acopy) (Variables|Default|GetImpact%20Normals) _array_index))
          (elif (Utilities|Enum|Equal(Enum) _array_element "SurfaceType3")
            (Utilities|Array|Add (Variables|Default|GetGlassImpacts) (Utilities|Array|Get(acopy) (Variables|Default|GetImpact%20Positions) _array_index))
            (Utilities|Array|Add (Variables|Default|GetGlassNormals) (Utilities|Array|Get(acopy) (Variables|Default|GetImpact%20Normals) _array_index))))))))