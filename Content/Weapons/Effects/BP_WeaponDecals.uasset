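; BP_WeaponDecals spawns impact decals for weapon hits through a single reused Niagara system.
; WeaponFired strips hits on default and SurfaceType1 surfaces, then passes positions, normals, surface types, hit count and muzzle position to Niagara user parameters.
; Flipping a boolean trigger signals each new shot, and the system respawns only when invalid or inactive.
; A retriggerable delay polls the system and destroys the actor once it is gone.
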(event Custom|WeaponFired
  (params (ImpactPositions :type Array%20of%20Vectors) (ImpactNormals :type Array%20of%20Vectors) (ImpactSurfaces :type Array%20of%20EPhysicalSurface%20Enums :default "SurfaceType_Default") (MuzzlePosition :type Vector))
  (Variables|Default|SetImpact%20Positions ImpactPositions)
  (Variables|Default|SetImpact%20Normals ImpactNormals)
  (Variables|Default|SetImpact%20Surfaces ImpactSurfaces)
  (Variables|Default|SetMuzzle%20Position MuzzlePosition)
  (CallFunction|RemoveInvalidSurfaces)
  (Utilities|FlowControl|Sequence
    (:then_0
      (Utilities|IsValid (Variables|Default|GetNS_Decals)
        (:Is%20Valid
          (if (Components|Activation|IsActive (Variables|Default|GetNS_Decals))
            _
            (else
              (bind _returnvalue (Niagara|SpawnSystematLocation "/Game/Effects/Particles/Impacts/NS_ImpactDecals.NS_ImpactDecals" "0, 0, 0" :!label _label))
              (Variables|Default|SetNS_Decals _returnvalue)
              (Variables|Default|SetDecalTrigger false))))
        (:Is%20Not%20Valid
          (goto _label)))
      (Variables|Default|SetDecalTrigger (not (Variables|Default|GetDecalTrigger)))
      (for (_array_element _array_index) (Variables|Default|GetImpact%20Surfaces)
        (Utilities|Array|SetArrayElem (Variables|Default|GetImpactSurfacesInt) _array_index (Math|Conversions|ToInteger(Byte) _array_element) true))
      (Class|NiagaraDataInterfaceArrayFunctionLibrary|SetNiagaraArrayInt32 (Variables|Default|GetNS_Decals) "User.ImpactSurfaces" (Variables|Default|GetImpactSurfacesInt))
      (Class|NiagaraDataInterfaceArrayFunctionLibrary|SetNiagaraArrayPosition (Variables|Default|GetNS_Decals) "User.ImpactPositions" (Variables|Default|GetImpact%20Positions))
      (Class|NiagaraDataInterfaceArrayFunctionLibrary|SetNiagaraArrayVector (Variables|Default|GetNS_Decals) "User.ImpactNormals" (Variables|Default|GetImpact%20Normals))
      (Class|NiagaraComponent|SetVariableInt (Variables|Default|GetNS_Decals) "User.NumberOfHits" (Utilities|Array|Length (Variables|Default|GetImpact%20Positions)))
      (Class|NiagaraComponent|SetVariablePosition (Variables|Default|GetNS_Decals) "User.MuzzlePosition" (Variables|Default|GetMuzzle%20Position))
      (Class|NiagaraComponent|SetVariableBool (Variables|Default|GetNS_Decals) "User.Trigger" (Variables|Default|GetDecalTrigger)))
    (:then_1
      (Utilities|FlowControl|RetriggerableDelay 0.2 :!label _label_2)
      (if (Utilities|IsValid (Variables|Default|GetNS_Decals))
        (goto _label_2)
        (else
          (Actor|DestroyActor))))))

(fn ConstructionScript)

(fn RemoveInvalidSurfaces
  (bind _output_get (LocalVariables|SetLcl_ImpactSurfaces (Variables|Default|GetImpact%20Surfaces)))
  (bind (_arrayindex _arrayelement) (Utilities|Array|ReverseforEachLoop _output_get)
    (:LoopBody
      (if (or (Utilities|Enum|Equal(Enum) _arrayelement "SurfaceType_Default") (Utilities|Enum|Equal(Enum) _arrayelement "SurfaceType1"))
        (Utilities|Array|RemoveIndex (Variables|Default|GetImpact%20Surfaces) _arrayindex)
        (Utilities|Array|RemoveIndex (Variables|Default|GetImpact%20Positions) _arrayindex)
        (Utilities|Array|RemoveIndex (Variables|Default|GetImpact%20Normals) _arrayindex)))
    (:Completed
      (return))))