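; Rifle enemy that attacks its AI controller's target with hitscan fire during an attack montage.
; Attack traces from the muzzle straight at the target once per pellet, applying and reporting damage, then signals attack end.
; DeployHitScanFiredFX also damages blocking hits and drives lazily spawned, reused muzzle/tracer, decal, impact and sound actors.
; It also supplies ideal ranges and maps movement speed to walk speed and ADS animation.
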(event EventBeginPlay
  (|CallParentFunction))

(event Collision|EventActorBeginOverlap
  (params (OtherActor :type Actor%20Object%20Reference)))

(event EventTick
  (params (DeltaSeconds :type Float%20%28single-precision%29)))

(event EventAttack
  (Animation|Montage|PlayMontage (Variables|Character|GetMesh) (Variables|Default|GetWeaponAttackMontage)
    (:then
      (bind _asaic_enemy_base (Utilities|Casting|CastToAIC_Enemy_Base (AI|GetAIController self)))
      (bind _attack_target (Variables|/Game/Enemies/AI/AIC_Enemy_Base.AIC_Enemy_Base_C|GetAttack%20Target _asaic_enemy_base)
        (:then
          (bind _result (Math|Integer|DecrementInt (Variables|/Script/Octahedron.TP_WeaponComponent|GetPellets (Variables|Default|GetWeaponComponent)))
            (:%20%20
              (for _index (range 0 (Math|Integer|Max(Integer) _result))
                (bind _outhit (Collision|LineTraceByChannel (Transformation|GetSocketLocation (Variables|Default|GetWeaponComponent) "Muzzle") (Transformation|GetActorLocation _attack_target) "TraceTypeQuery3" false 0 "None" true "(R=1.000000,G=0.000000,B=0.000000,A=1.000000)" "(R=0.000000,G=1.000000,B=0.000000,A=1.000000)" 2.0))
                (CallFunction|DeployHitScanFiredFX (Utilities|Array|MakeArray _outhit))
                (Class|BPIDamagable|TakeDamage(Message) (.HitActor (Collision|BreakHitResult _outhit)) (Utilities|Struct|MakeS_DamageInfo 2e+01 "NewEnumerator2" "NewEnumerator1" false false false false (.Location (Collision|BreakHitResult _outhit))) self)
                (Class|AISenseDamage|ReportDamageEvent _attack_target self 2e+01 (Transformation|GetActorLocation) "0, 0, 0" "None")))))
        (:else)))
    (:OnCompleted
      (Default|CallOnAttackEnd :!label _label))
    (:OnInterrupted
      (goto _label))))

(fn ConstructionScript
  (|CallParentFunction))

(fn SetMovementSpeed
  (params (Speed :type E_MovementSpeed%20Enum :default "NewEnumerator0"))
  (bind _asabp_mannequin_base (Utilities|Casting|CastToABP_Mannequin_Base (Components|SkeletalMesh|GetAnimInstance (Variables|Character|GetMesh))))
  (Variables|/Game/Characters/Heroes/Mannequin/Animations/ABP_Mannequin_Base.ABP_Mannequin_Base_C|SetGameplayTag_IsADS _asabp_mannequin_base (Utilities|Enum|Equal(Enum) Speed "NewEnumerator1"))
  (Variables|/Script/Engine.CharacterMovementComponent|SetMaxWalkSpeed (Variables|Character|GetCharacterMovement) (Utilities|Select :Index Speed :NewEnumerator0 0.0 :NewEnumerator1 2e+02 :NewEnumerator2 6e+02 :NewEnumerator3 7.5e+02))
  (return 0.0))

(fn GetIdealRange
  (return 6e+02 6e+02))

(fn DeployHitScanFiredFX
  (params (HitResults :type Array%20of%20Hit%20Result%20Structures))
  (bind _returnvalue (Components|GetOwner))
  (bind _weaponcomponent (Variables|Default|GetWeaponComponent))
  (bind _weaponcomponent_2 (Variables|Default|GetWeaponComponent))
  (bind _weaponcomponent_3 (Variables|Default|GetWeaponComponent))
  (Utilities|FlowControl|Sequence
    (:then_0
      ;[1 1 1] Save hit result Info and apply damage if applicable
      (Utilities|Array|Clear (LocalVariables|GetImpact%20Positions))
      (Utilities|Array|Clear (LocalVariables|GetImpact%20Normals))
      (Utilities|Array|Clear (LocalVariables|GetImpactSurfaceTypes))
      (Utilities|Array|Clear (LocalVariables|GetTracerPositions))
      (for _array_element HitResults
        (if (.bBlockingHit (Collision|BreakHitResult _array_element))
          (Utilities|Array|Add (LocalVariables|GetTracerPositions) (.Location (Collision|BreakHitResult _array_element)))
          (Utilities|Array|Add (LocalVariables|GetImpact%20Positions) (.Location (Collision|BreakHitResult _array_element)))
          (Utilities|Array|Add (LocalVariables|GetImpact%20Normals) (.Normal (Collision|BreakHitResult _array_element)))
          (Utilities|Array|Add (LocalVariables|GetImpactSurfaceTypes) (Variables|/Script/PhysicsCore.PhysicalMaterial|GetSurfaceType (.PhysMat (Collision|BreakHitResult _array_element))))
          (Class|BPIDamagable|TakeDamage(Message) (.HitActor (Collision|BreakHitResult _array_element)) (Utilities|Struct|MakeS_DamageInfo (Variables|/Script/Octahedron.TP_WeaponComponent|GetDamage (Variables|Default|GetWeaponComponent)) "NewEnumerator2" "NewEnumerator1" false false false false (.Normal (Collision|BreakHitResult _array_element))) _returnvalue)
          (Class|AISenseDamage|ReportDamageEvent (.HitActor (Collision|BreakHitResult _array_element)) _returnvalue (Variables|/Script/Octahedron.TP_WeaponComponent|GetDamage (Variables|Default|GetWeaponComponent)) (Transformation|GetActorLocation (Components|GetOwner)) "0, 0, 0" "None")
          (else
            (Utilities|Array|Add (LocalVariables|GetTracerPositions) (.TraceEnd (Collision|BreakHitResult _array_element))))))
      (LocalVariables|SetMuzzle%20Position (Transformation|GetSocketLocation _weaponcomponent (Variables|/Script/Octahedron.TP_WeaponComponent|GetMuzzleSocketName _weaponcomponent))))
    (:then_1
      ;[1 1 1] Muzzle Flash, Tracer, and Shell Eject
      (Utilities|IsValid (Variables|Default|GetBP_WeaponFX)
        (:Is%20Valid
          _)
        (:Is%20Not%20Valid
          (bind _returnvalue_2 (Game|SpawnActorfromClass "/Game/Weapons/Effects/BP_WeaponFX.BP_WeaponFX_C" (Math|Transform|MakeTransform "0, 0, 0") "Undefined" "MultiplyWithRoot" 0 (Variables|Default|GetWeaponComponent) (Variables|/Script/Octahedron.TP_WeaponComponent|GetMuzzleFlash_FX _weaponcomponent_2) (Variables|/Script/Octahedron.TP_WeaponComponent|GetTracer_FX _weaponcomponent_2) (Variables|/Script/Octahedron.TP_WeaponComponent|GetShellEjectMesh _weaponcomponent_2) (Variables|/Script/Octahedron.TP_WeaponComponent|GetMuzzleSocketName _weaponcomponent_2) (Variables|/Script/Octahedron.TP_WeaponComponent|GetShellEjectSocketName _weaponcomponent_2) 0))
          (bind _output_get (Variables|Default|SetBP_WeaponFX _returnvalue_2))
          (Transformation|AttachComponentToComponent _output_get (Variables|Default|GetWeaponComponent) "None" "KeepRelative" "KeepRelative" "KeepRelative" true)))
      (Default|WeaponFired (Variables|Default|GetBP_WeaponFX) (LocalVariables|GetTracerPositions)))
    (:then_2
      ;[1 1 1] Bullet Decals
      (Utilities|IsValid (Variables|Default|GetBP_WeaponDecalsFX)
        (:Is%20Valid
          _)
        (:Is%20Not%20Valid
          (bind _returnvalue_3 (Game|SpawnActorfromClass "/Game/Weapons/Effects/BP_WeaponDecals.BP_WeaponDecals_C" (Math|Transform|MakeTransform "0, 0, 0") "Undefined" "MultiplyWithRoot" 0 0))
          (bind _output_get_2 (Variables|Default|SetBP_WeaponDecalsFX _returnvalue_3))
          (Transformation|AttachComponentToComponent _output_get_2 (Variables|Default|GetWeaponComponent) "None" "KeepRelative" "KeepRelative" "KeepRelative" true)))
      (Default|WeaponFired (Variables|Default|GetBP_WeaponDecalsFX) (LocalVariables|GetImpact%20Positions) (LocalVariables|GetImpact%20Normals) (LocalVariables|GetImpactSurfaceTypes) (LocalVariables|GetMuzzle%20Position)))
    (:then_3
      ;[1 1 1] Weapon Impact
      (if (Utilities|Array|IsNotEmpty (LocalVariables|GetImpact%20Positions))
        (Utilities|IsValid (Variables|Default|GetBP_WeaponImpactsFX)
          (:Is%20Valid
            _)
          (:Is%20Not%20Valid
            (bind _returnvalue_4 (Game|SpawnActorfromClass "/Game/Weapons/Effects/BP_WeaponImpacts.BP_WeaponImpacts_C" (Math|Transform|MakeTransform "0, 0, 0") "Undefined" "MultiplyWithRoot" 0 0))
            (bind _output_get_3 (Variables|Default|SetBP_WeaponImpactsFX _returnvalue_4))
            (Transformation|AttachComponentToComponent _output_get_3 (Variables|Default|GetWeaponComponent) "None" "KeepRelative" "KeepRelative" "KeepRelative" true)))
        (Default|WeaponFired (Variables|Default|GetBP_WeaponImpactsFX) (LocalVariables|GetImpact%20Positions) (LocalVariables|GetImpact%20Normals) (LocalVariables|GetImpactSurfaceTypes) (LocalVariables|GetMuzzle%20Position))))
    (:then_4
      ;[1 1 1] Weapon Fire Sounds
      (Utilities|IsValid (Variables|Default|GetWeaponSounds)
        (:Is%20Valid
          _)
        (:Is%20Not%20Valid
          (bind _returnvalue_5 (Game|SpawnActorfromClass "/Game/Effects/Blueprints/B_WeaponSounds.B_WeaponSounds_C" (Math|Transform|MakeTransform "0, 0, 0") "Undefined" "MultiplyWithRoot" 0 (Variables|Default|GetWeaponComponent) (* (Variables|/Script/Octahedron.TP_WeaponComponent|GetFireDelay _weaponcomponent_3) (Variables|/Script/Octahedron.TP_WeaponComponent|GetFireSoundDelayScale _weaponcomponent_3)) (Variables|/Script/Octahedron.TP_WeaponComponent|GetFireSound (Variables|Default|GetWeaponComponent)) 0))
          (bind _output_get_4 (Variables|Default|SetWeaponSounds _returnvalue_5))
          (Transformation|AttachComponentToComponent _output_get_4 (Variables|Default|GetWeaponComponent) "None" "KeepRelative" "KeepRelative" "KeepRelative" true)))
      (Default|Fire (Variables|Default|GetWeaponSounds)))))