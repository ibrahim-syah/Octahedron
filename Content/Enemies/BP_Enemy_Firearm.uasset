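; Firearm-wielding enemy Blueprint that fires its current weapon on Attack and supplies movement speed and ideal combat range.
; Attack skips when the weapon is busy or cooling down, plays a dry-fire sound and reloads if ammo remains when the magazine is empty.
; Otherwise it fires by mode, using looping timers for burst and auto.
; SetMovementSpeed maps movement states to walk speeds and flags aim-down-sights on the anim instance when walking.
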(event Custom|StartBurstFire
  (Class|TPWeaponComponent|BurstFire (Variables|Default|GetCurrentWeapon)))

(event Custom|StartAutoFire
  (Class|TPWeaponComponent|FullAutoFire (Variables|Default|GetCurrentWeapon)))

(event EventBeginPlay
  (|CallParentFunction))

(event Collision|EventActorBeginOverlap
  (params (OtherActor :type Actor%20Object%20Reference)))

(event EventTick
  (params (DeltaSeconds :type Float%20%28single-precision%29)))

(event EventAttack
  (bind _currentweapon (Variables|Default|GetCurrentWeapon))
  (bind _currentweapon_2 (Variables|Default|GetCurrentWeapon))
  (Variables|/Script/Octahedron.TP_WeaponComponent|SetIsWielderHoldingShootButton (Variables|Default|GetCurrentWeapon) true)
  (if (not (Math|Boolean|ORBoolean (Variables|/Script/Octahedron.TP_WeaponComponent|GetIsReloading _currentweapon) (Variables|/Script/Octahedron.TP_WeaponComponent|GetIsStowing _currentweapon) (Variables|/Script/Octahedron.TP_WeaponComponent|GetIsEquipping _currentweapon) (> (Utilities|Time|GetTimerRemainingTimebyHandle (Variables|/Script/Octahedron.TP_WeaponComponent|GetFireRateDelayTimerHandle _currentweapon)) 0.0)))
    (if (<= (Variables|/Script/Octahedron.TP_WeaponComponent|GetCurrentMagazineCount (Variables|Default|GetCurrentWeapon)) 0)
      (Class|TPWeaponComponent|StopFire (Variables|Default|GetCurrentWeapon))
      (Variables|/Script/Octahedron.TP_WeaponComponent|SetIsWielderHoldingShootButton (Variables|Default|GetCurrentWeapon) false)
      (Audio|SpawnSoundAttached (Variables|/Script/Octahedron.TP_WeaponComponent|GetDryFireSound _currentweapon_2) _currentweapon_2 "None" "0, 0, 0" "0, 0, 0" "KeepRelativeOffset" false 1.0 1.0 0.0 0 0)
      (bind _returnvalue (Class|WeaponWielderInterface|GetRemainingAmmo(Message) self))
      (if (> _returnvalue 0)
        (Class|TPWeaponComponent|Reload (Variables|Default|GetCurrentWeapon)))
      (else
        (Utilities|Time|ClearandInvalidateTimerbyHandle (Variables|/Script/Octahedron.TP_WeaponComponent|GetFireRateDelayTimerHandle (Variables|Default|GetCurrentWeapon)))
        (switch Utilities|FlowControl|Switch|SwitchonEFireMode (Variables|/Script/Octahedron.TP_WeaponComponent|GetFireMode (Variables|Default|GetCurrentWeapon))
          (:Single
            (Class|TPWeaponComponent|SingleFire (Variables|Default|GetCurrentWeapon))
            (bind _returnvalue_2 (Utilities|Time|SetTimerbyEvent 0 (Variables|/Script/Octahedron.TP_WeaponComponent|GetFireDelay (Variables|Default|GetCurrentWeapon))))
            (Variables|/Script/Octahedron.TP_WeaponComponent|SetFireRateDelayTimerHandle (Variables|Default|GetCurrentWeapon) _returnvalue_2))
          (:Burst
            (bind _returnvalue_3 (Utilities|Time|SetTimerbyEvent (delegate Custom|StartBurstFire) (Variables|/Script/Octahedron.TP_WeaponComponent|GetFireDelay (Variables|Default|GetCurrentWeapon)) true))
            (Variables|/Script/Octahedron.TP_WeaponComponent|SetFireRateDelayTimerHandle (Variables|Default|GetCurrentWeapon) _returnvalue_3))
          (:Auto
            (bind _returnvalue_4 (Utilities|Time|SetTimerbyEvent (delegate Custom|StartAutoFire) (Variables|/Script/Octahedron.TP_WeaponComponent|GetFireDelay (Variables|Default|GetCurrentWeapon)) true))
            (Variables|/Script/Octahedron.TP_WeaponComponent|SetFireRateDelayTimerHandle (Variables|Default|GetCurrentWeapon) _returnvalue_4)))))))

(fn ConstructionScript
  (|CallParentFunction))

(fn SetMovementSpeed
  (params (Speed :type E_MovementSpeed%20Enum :default "NewEnumerator0"))
  (bind _asabp_mannequin_base (Utilities|Casting|CastToABP_Mannequin_Base (Components|SkeletalMesh|GetAnimInstance (Variables|Character|GetMesh))))
  (Variables|/Game/Characters/Heroes/Mannequin/Animations/ABP_Mannequin_Base.ABP_Mannequin_Base_C|SetGameplayTag_IsADS _asabp_mannequin_base (Utilities|Enum|Equal(Enum) Speed "NewEnumerator1"))
  (Variables|/Script/Engine.CharacterMovementComponent|SetMaxWalkSpeed (Variables|Character|GetCharacterMovement) (Utilities|Select :Index Speed :NewEnumerator0 0.0 :NewEnumerator1 2e+02 :NewEnumerator2 6e+02 :NewEnumerator3 7.5e+02))
  (return 0.0))

(fn GetIdealRange
  (return 6e+02 6e+02))