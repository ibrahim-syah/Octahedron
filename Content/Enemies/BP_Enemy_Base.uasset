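; Base enemy character that fights with pooled weapons and melee, driven by its AIC_Enemy_Base controller.
; BPC damage system feeds health and hit responses: directional hit reactions, staggers or knockback launches that switch the AI state.
; A timed-fade health bar shows on damage; death triggers ragdoll and a Niagara cube effect before destruction.
; Weapons attach with linked anim layers, and melee sphere-traces on a montage notify.
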(event Custom|Die
  (bind _aic_enemy_base (Variables|AI|GetAIC%20Enemy%20Base))
  (Components|Movement|StopMovementImmediately (Variables|Character|GetCharacterMovement))
  (Components|DestroyComponent (Variables|Default|GetHealthBar))
  (Physics|SetSimulatePhysics (Variables|Character|GetMesh) true)
  (Collision|SetCollisionEnabled (Variables|Character|GetMesh) "QueryAndPhysics")
  (AI|Logic|StopLogic (Variables|/Script/AIModule.AIController|GetBrainComponent _aic_enemy_base) "")
  (Default|SetStateasDead _aic_enemy_base)
  (bind _returnvalue (Niagara|SpawnSystemAttached "/Game/Effects/Particles/Impacts/NS_DeathCubes.NS_DeathCubes" (Variables|Character|GetMesh) "None" "0, 0, 0" "0, 0, 0" "KeepRelativeOffset" false false))
  (Niagara|SetNiagaraVariable(Float) _returnvalue "KillTimeLength" 2.0)
  (Niagara|SetNiagaraVariable(Vector3) _returnvalue "BodyColor" (Math|Conversions|ToVector(LinearColor) (Class|KismetMathLibrary|LinearColorRed)))
  (EventDispatchers|AssignOnSystemFinished _returnvalue (delegate Custom|OnSystemFinished_Event))
  (Components|Activation|Activate _returnvalue true))

(event Custom|RespondDamage
  (params (DamageResponse :type E_DamageResponse%20Enum :default "NewEnumerator0") (DamageCauser :type Actor%20Object%20Reference) (KnockbackEpicenter :type Vector) (HitBoneName :type Name) (DamageDirection :type E_DamageDirection%20Enum :default "NewEnumerator0"))
  (bind _returnvalue (Math|Random|RandomIntegerinRange 0 1))
  (bind _healthbar (Variables|Default|GetHealthBar))
  (if (Variables|/Script/Engine.SceneComponent|GetbVisible (Variables|Default|GetHealthBar))
    _
    (else
      (Rendering|SetVisibility _healthbar true false)
      (bind _asw_dynamic_health_bar (Utilities|Casting|CastToW_DynamicHealthBar (UserInterface|GetWidget _healthbar)))
      (UserInterface|Animation|PlayAnimation _asw_dynamic_health_bar (Variables|/Game/UI/Hud/Widgets/HealthBar/W_DynamicHealthBar.W_DynamicHealthBar_C|GetFadeIn _asw_dynamic_health_bar) 0.0 1 "Forward" 1.0 false)))
  (Utilities|FlowControl|Sequence
    (:then_0
      (Utilities|FlowControl|RetriggerableDelay 1e+01)
      (bind _healthbar_2 (Variables|Default|GetHealthBar)
        (:then
          (bind _asw_dynamic_health_bar_2 (Utilities|Casting|CastToW_DynamicHealthBar (UserInterface|GetWidget _healthbar_2)))
          (Class|UserWidget|BindtoAnimationFinished _asw_dynamic_health_bar_2 (Variables|/Game/UI/Hud/Widgets/HealthBar/W_DynamicHealthBar.W_DynamicHealthBar_C|GetFadeOut _asw_dynamic_health_bar_2) (delegate Custom|SetVisibilityFalse))
          (UserInterface|Animation|PlayAnimation _asw_dynamic_health_bar_2 (Variables|/Game/UI/Hud/Widgets/HealthBar/W_DynamicHealthBar.W_DynamicHealthBar_C|GetFadeOut _asw_dynamic_health_bar_2) 0.0 1 "Forward" 1.0 false))
        (:else)))
    (:then_1
      (switch Utilities|FlowControl|Switch|SwitchonE_DamageResponse DamageResponse
        (:NewEnumerator1
          (Animation|Montage|PlayMontage (Variables|Character|GetMesh) (Utilities|Select :Index DamageDirection :NewEnumerator0 "/Game/Characters/Heroes/Mannequin/Animations/Actions/AM_MM_HitReact_Front_Lgt_01.AM_MM_HitReact_Front_Lgt_01" :NewEnumerator1 (Utilities|Select :Index (Math|Random|RandomIntegerinRange 0 3) :Option%200 "/Game/Characters/Heroes/Mannequin/Animations/Actions/AM_MM_HitReact_Front_Lgt_01.AM_MM_HitReact_Front_Lgt_01" :Option%201 "/Game/Characters/Heroes/Mannequin/Animations/Actions/AM_MM_HitReact_Front_Lgt_02.AM_MM_HitReact_Front_Lgt_02" :Option%202 "/Game/Characters/Heroes/Mannequin/Animations/Actions/AM_MM_HitReact_Front_Med_01.AM_MM_HitReact_Front_Med_01" :Option%203 "/Game/Characters/Heroes/Mannequin/Animations/Actions/AM_MM_HitReact_Front_Med_02.AM_MM_HitReact_Front_Med_02") :NewEnumerator2 (Utilities|Select :Index (Math|Random|RandomIntegerinRange 0 1) :Option%200 "/Game/Characters/Heroes/Mannequin/Animations/Actions/AM_MM_HitReact_Back_Lgt_01.AM_MM_HitReact_Back_Lgt_01" :Option%201 "/Game/Characters/Heroes/Mannequin/Animations/Actions/AM_MM_HitReact_Back_Med_01.AM_MM_HitReact_Back_Med_01") :NewEnumerator3 (Utilities|Select :Index _returnvalue :Option%200 "/Game/Characters/Heroes/Mannequin/Animations/Actions/AM_MM_HitReact_Left_Lgt_01.AM_MM_HitReact_Left_Lgt_01" :Option%201 "/Game/Characters/Heroes/Mannequin/Animations/Actions/AM_MM_HitReact_Left_Med_01.AM_MM_HitReact_Left_Med_01") :NewEnumerator4 (Utilities|Select :Index _returnvalue :Option%200 "/Game/Characters/Heroes/Mannequin/Animations/Actions/AM_MM_HitReact_Right_Lgt_01.AM_MM_HitReact_Right_Lgt_01" :Option%201 "/Game/Characters/Heroes/Mannequin/Animations/Actions/AM_MM_HitReact_Right_Med_01.AM_MM_HitReact_Right_Med_01"))))
        (:NewEnumerator2
          (Components|Movement|StopMovementImmediately (Variables|Character|GetCharacterMovement))
          (Default|SetStateasFrozen (Variables|AI|GetAIC%20Enemy%20Base))
          (Animation|Montage|PlayMontage (Variables|Character|GetMesh) "/Game/Characters/Heroes/Mannequin/Animations/Actions/AM_MM_Staggered.AM_MM_Staggered"
            (:OnCompleted
              (Default|SetStateasAttacking (Variables|AI|GetAIC%20Enemy%20Base) DamageCauser true))
            (:OnInterrupted
              (bind _aic_enemy_base (Variables|AI|GetAIC%20Enemy%20Base)
                (:then
                  (Default|SetStateasAttacking _aic_enemy_base DamageCauser true))
                (:else)))))
        (:NewEnumerator4
          (Animation|Montage|PlayMontage (Variables|Character|GetMesh) "/Game/Characters/Heroes/Mannequin/Animations/Actions/AM_MM_HitReact_Front_Hvy_01.AM_MM_HitReact_Front_Hvy_01"
            (:then
              (Character|LaunchCharacter (* (Math|Vector|Normalize (- (Transformation|GetActorLocation) KnockbackEpicenter)) 1.5e+03) true true)
              (Default|SetStateasAttacking (Variables|AI|GetAIC%20Enemy%20Base) 0 true))))))))

(event Custom|OnSystemFinished_Event
  (params (PSystem :type Niagara%20Component%20Object%20Reference))
  (Actor|DestroyActor))

(event Custom|UpdateHealthBarWorld
  (bind _healthbar (Variables|Default|GetHealthBar)
    (:then
      (Transformation|SetWorldRotation _healthbar (Math|Rotator|MakeRotator 0.0 0.0 (.yaw (Math|Rotator|FindLookatRotation (Transformation|GetWorldLocation _healthbar) (Transformation|GetWorldLocation (Variables|/Script/Engine.PlayerCameraManager|GetTransformComponent (Game|GetPlayerCameraManager 0)))))) false false))
    (:else)))

(event Custom|SetVisibilityFalse
  (Rendering|SetVisibility (Variables|Default|GetHealthBar) false false))

(event EventBeginPlay
  (bind _asaic_enemy_base (Utilities|Casting|CastToAIC_Enemy_Base (AI|GetAIController self)))
  (Variables|AI|SetAIC%20Enemy%20Base _asaic_enemy_base)
  (EventDispatchers|BindEventtoOnDeath (Variables|Default|GetBPC_DamageSystem) (EventDispatchers|CreateEvent :!event Custom|Die))
  (EventDispatchers|BindEventtoOnDamageResponse (Variables|Default|GetBPC_DamageSystem) (EventDispatchers|CreateEvent :!event Custom|RespondDamage))
  (bind _returnvalue (UserInterface|CreateWidget "/Game/UI/Hud/Widgets/HealthBar/W_DynamicHealthBar.W_DynamicHealthBar_C"))
  (bind _maxhealth (CallFunction|GetMaxHealth))
  (bind _health (CallFunction|GetCurrentHealth))
  (Default|UpdateValues _returnvalue (/ _health _maxhealth))
  (Utilities|Time|SetTimerbyEvent (EventDispatchers|CreateEvent :!event Custom|UpdateHealthBarWorld) 0.016667 true)
  (UserInterface|SetWidget (Variables|Default|GetHealthBar) _returnvalue)
  (Components|SkeletalMesh|AnimationBlueprintLinking|LinkAnimClassLayers (Variables|Character|GetMesh) "/Game/Characters/Heroes/Mannequin/Animations/Locomotion/Unarmed/ABP_UnarmedAnimLayers.ABP_UnarmedAnimLayers_C"))

(event EventUnequipWeapon
  (Variables|Default|GetCurrentWeapon
    (:then
      (CallFunction|DetachWeapon)
      (Components|SkeletalMesh|AnimationBlueprintLinking|LinkAnimClassLayers (Variables|Character|GetMesh) "/Game/Characters/Heroes/Mannequin/Animations/Locomotion/Unarmed/ABP_UnarmedAnimLayers.ABP_UnarmedAnimLayers_C")
      (Variables|Weapon|SetIsWeaponEquipped false)
      (Default|CallOnWeaponUnequipped))
    (:else)))

(event EventOnReloadSuccess
  (bind _currentweapon (Variables|Default|GetCurrentWeapon))
  (Class|TPWeaponComponent|OnReloaded _currentweapon)
  (Class|TPWeaponComponent|SetIsReloadingFalse _currentweapon))

(event EventEquipWeapon
  (bind _currentweapon (Variables|Default|GetCurrentWeapon)
    (:then
      (if (Utilities|Enum|NotEqual(Enum) (Variables|/Script/Octahedron.TP_WeaponComponent|GetAmmoType _currentweapon) "Primary")
        (bind _returnvalue (CallFunction|InstantDetachWeapon))
        ;[1 1 1] Check if succesfully detached
        (if _returnvalue
          (Default|SpawnfromPool (Variables|Default|GetAC_WeaponPool) 0 :!label _label)
          (Variables|Weapon|SetIsWeaponEquipped true)
          (Default|CallOnWeaponEquipped))))
    (:else
      (goto _label))))

(event EventAttack
  (bind _notifyname (Animation|Montage|PlayMontage (Variables|Character|GetMesh) (Variables|/Script/Octahedron.TP_WeaponComponent|GetTPMeleeAnimation (Variables|Default|GetCurrentWeapon)))
    (:then
      (Variables|/Game/DamageSystem/BPC_DamageSystem.BPC_DamageSystem_C|SetIsInterruptable (Variables|Default|GetBPC_DamageSystem) false))
    (:OnCompleted
      (Default|CallOnAttackEnd :!label _label)
      (Variables|/Game/DamageSystem/BPC_DamageSystem.BPC_DamageSystem_C|SetIsInterruptable (Variables|Default|GetBPC_DamageSystem) true))
    (:OnInterrupted
      (goto _label))
    (:OnNotifyBegin
      (if (== _notifyname "Melee")
        (CallFunction|SphereTraceMelee)))))

(event EventDetachWeapon
  (if (not (Math|Boolean|ORBoolean (not (Variables|Default|GetbHasWeapon)) (Variables|/Script/Octahedron.TP_WeaponComponent|GetIsReloading (Variables|Default|GetCurrentWeapon)) (Variables|/Script/Octahedron.TP_WeaponComponent|GetIsStowing (Variables|Default|GetCurrentWeapon)) (Variables|/Script/Octahedron.TP_WeaponComponent|GetIsEquipping (Variables|Default|GetCurrentWeapon)) (> (Utilities|Time|GetTimerRemainingTimebyHandle (Variables|/Script/Octahedron.TP_WeaponComponent|GetFireRateDelayTimerHandle (Variables|Default|GetCurrentWeapon))) 0.0)))
    (bind _currentweapon (Variables|Default|GetCurrentWeapon)
      (:then
        (Variables|/Script/Octahedron.TP_WeaponComponent|SetIsStowing _currentweapon true)
        (Components|Timeline|SetNewTime (Variables|/Script/Octahedron.TP_WeaponComponent|GetADSTL _currentweapon) 0.0)
        (Audio|Components|Audio|Stop (Variables|/Script/Octahedron.TP_WeaponComponent|GetADSTL _currentweapon))
        (Animation|Montage|PlayMontage (Variables|Character|GetMesh) "/Game/Characters/Heroes/Mannequin/Animations/Actions/AM_MM_Generic_Unequip.AM_MM_Generic_Unequip"
          (:then
            (Class|TPWeaponComponent|Stow _currentweapon)
            (Variables|Default|SetbHasWeapon false)
            (Variables|Default|SetCurrentWeapon 0))))
      (:else))))

(event EventOnWeaponReload
  (Animation|Montage|PlayMontage (Variables|Character|GetMesh) (Variables|/Script/Octahedron.TP_WeaponComponent|GetTPReloadAnimation (Variables|Default|GetCurrentWeapon))))

(event EventOnWeaponFired
  (Animation|Montage|PlayMontage (Variables|Character|GetMesh) "/Game/Weapons/Pistol/Animations/MM_Pistol_Fire_Montage.MM_Pistol_Fire_Montage"
    (:then
      (Class|Actor|MakeNoise 1.0 self (Transformation|GetWorldLocation (Variables|Default|GetCurrentWeapon)) 0.0 "None"))))

(event EventOnWeaponStopReloadAnimation
  (params (blendTime :type Float%20%28single-precision%29))
  (Animation|Montage|MontageStop (Components|SkeletalMesh|GetAnimInstance (Variables|Character|GetMesh)) blendTime (Variables|/Script/Octahedron.TP_WeaponComponent|GetTPReloadAnimation (Variables|Default|GetCurrentWeapon))))

(event EventAttachWeapon
  (params (Weapon :type TP%20Weapon%20Component%20Object%20Reference))
  (Class|TPWeaponComponent|SetOwningWeaponWielder Weapon self)
  (if (not (== (Variables|Default|GetCurrentWeapon) Weapon))
    (Class|TPWeaponComponent|SetIsEquippingFalse Weapon)
    (Variables|/Script/Octahedron.TP_WeaponComponent|SetIsEquipping Weapon true)
    (Transformation|AttachComponentToComponent Weapon (Variables|Character|GetMesh) "weapon_r" "SnapToTarget" "SnapToTarget" "SnapToTarget" true)
    (bind _output_get (Variables|Default|SetCurrentWeapon Weapon))
    (Transformation|AddRelativeRotation _output_get (.rotation (Variables|/Script/Octahedron.TP_WeaponComponent|GetTPTransform _output_get)) false false)
    (Class|TPWeaponComponent|Equip _output_get)
    (Components|SkeletalMesh|AnimationBlueprintLinking|LinkAnimClassLayers (Variables|Character|GetMesh) (Variables|Weapon|GetWeaponAnimLayer))
    (Animation|Montage|PlayMontage (Variables|Character|GetMesh) (Variables|/Script/Octahedron.TP_WeaponComponent|GetTPEquipAnimation (Variables|Default|GetCurrentWeapon))
      (:then
        (Default|CallOnEquipDelegate (Variables|Default|GetCurrentWeapon) self (Variables|Default|GetCurrentWeapon))
        (Variables|Default|SetbHasWeapon true)
        (Variables|/Script/Octahedron.TP_WeaponComponent|SetCanFire (Variables|Default|GetCurrentWeapon) true))
      (:OnBlendOut
        (Class|TPWeaponComponent|EquipAnimationBlendOut (Variables|Default|GetCurrentWeapon) (Variables|/Script/Octahedron.TP_WeaponComponent|GetTPEquipAnimation (Variables|Default|GetCurrentWeapon)) false)))))

(event EventOnStopFiring
  (Default|CallOnAttackEnd))

(fn ConstructionScript)

(fn SphereTraceMelee
  (bind _returnvalue (Transformation|GetActorLocation))
  (bind _instigator (Variables|Default|GetInstigator))
  (bind _attackrange (CallFunction|GetMeleeRange))
  (bind _outhit (Collision|SphereTraceForObjects _returnvalue (+ _returnvalue (* (Transformation|GetActorForwardVector) _attackrange)) 2e+01 (Utilities|Array|MakeArray "ObjectTypeQuery3") false (Utilities|Array|MakeArray self) "None" true "(R=1.000000,G=0.000000,B=0.000000,A=1.000000)" "(R=0.000000,G=1.000000,B=0.000000,A=1.000000)" 2.0))
  (if true
    (bind _finaldamage (Class|BPIDamagable|TakeDamage(Message) (.HitActor (Collision|BreakHitResult _outhit)) (Utilities|Struct|MakeS_DamageInfo 25.0 "NewEnumerator1" "NewEnumerator2" false false false false (.Location (Collision|BreakHitResult _outhit)) (.Normal (Collision|BreakHitResult _outhit)) (.HitBoneName (Collision|BreakHitResult _outhit)) 1.0) _instigator "0, 0, 0"))
    (Audio|SpawnSoundatLocation "/Game/Audio/MetaSounds/sfx_Weapon_MeleeImpact_nl_meta.sfx_Weapon_MeleeImpact_nl_meta" (.Location (Collision|BreakHitResult _outhit)) "0, 0, 0" 1.0 1.0 0.0 0 0)
    (Class|AISenseDamage|ReportDamageEvent (.HitActor (Collision|BreakHitResult _outhit)) _instigator _finaldamage (Transformation|GetActorLocation) "0, 0, 0" "None")
    (return false)))

(fn GetCurrentHealth
  (return (Variables|/Game/DamageSystem/BPC_DamageSystem.BPC_DamageSystem_C|GetHealth (Variables|Default|GetBPC_DamageSystem))))

(fn GetIdealRange
  (return 1e+02 3.5e+02))

(fn GetMaxHealth
  (return (Variables|/Game/DamageSystem/BPC_DamageSystem.BPC_DamageSystem_C|GetMaxHealth (Variables|Default|GetBPC_DamageSystem))))

(fn GetMeleeRange
  (return 2e+02))

(fn GetPatrolRoute
  (return (Variables|AI|GetPatrolRoute)))

(fn GetRemainingAmmo
  (switch Utilities|FlowControl|Switch|SwitchonEAmmoType (Variables|/Script/Octahedron.TP_WeaponComponent|GetAmmoType (Variables|Default|GetCurrentWeapon))
    (:None
      (return 0))
    (:Primary
      (return 999))
    (:Special
      (return (Variables|Default|GetSpecialAmmoRemaining)))
    (:Heavy
      (return (Variables|Default|GetHeavyAmmoRemaining)))))

(fn GetTraceForward
  (return (Math|Vector|GetForwardVector (Variables|Collision|GetCapsuleComponent))))

(fn GetTraceStart
  (return (Transformation|GetActorLocation)))

(fn GetWielderControlRotation
  (return (Pawn|GetControlRotation (Pawn|GetController) :!class /Script/Engine.Controller)))

(fn Heal
  (params (Amount :type Float%20%28double-precision%29))
  (bind _newhealth (Default|Heal (Variables|Default|GetBPC_DamageSystem) Amount))
  (bind _healthbar (Variables|Default|GetHealthBar)
    (:then
      (bind _maxhealth (CallFunction|GetMaxHealth))
      (bind _health (CallFunction|GetCurrentHealth))
      (bind _asw_dynamic_health_bar (Utilities|Casting|CastToW_DynamicHealthBar (UserInterface|GetWidget _healthbar))
        (:then
          (Default|UpdateValues _asw_dynamic_health_bar (/ _health _maxhealth)))
        (:CastFailed
          _)))
    (:else
      _))
  (return _newhealth))

(fn InstantDetachWeapon
  (if (Math|Boolean|ORBoolean (not (Variables|Default|GetbHasWeapon)) (Variables|/Script/Octahedron.TP_WeaponComponent|GetIsReloading (Variables|Default|GetCurrentWeapon)) (> (Utilities|Time|GetTimerRemainingTimebyHandle (Variables|/Script/Octahedron.TP_WeaponComponent|GetFireRateDelayTimerHandle (Variables|Default|GetCurrentWeapon))) 0.0))
    (return false)
    (else
      (bind _currentweapon (Variables|Default|GetCurrentWeapon)
        (:then
          (Variables|/Script/Octahedron.TP_WeaponComponent|SetIsStowing _currentweapon true)
          (Class|TPWeaponComponent|ExitADS _currentweapon true)
          (Transformation|DetachFromComponent _currentweapon "KeepRelative" "KeepRelative" "KeepRelative" true)
          (Variables|/Script/Octahedron.TP_WeaponComponent|SetCanFire _currentweapon false)
          (Variables|/Script/Octahedron.TP_WeaponComponent|SetIsStowing _currentweapon false)
          (Default|CallOnStowDelegate _currentweapon self _currentweapon)
          (Variables|Default|SetbHasWeapon false)
          (Variables|Default|SetCurrentWeapon 0)
          (return true))
        (:else)))))

(fn IsDead
  (return (Variables|/Game/DamageSystem/BPC_DamageSystem.BPC_DamageSystem_C|GetIsDead (Variables|Default|GetBPC_DamageSystem))))

(fn SetMovementSpeed
  (params (Speed :type E_MovementSpeed%20Enum :default "NewEnumerator0"))
  (bind _asabp_mannequin_base (Utilities|Casting|CastToABP_Mannequin_Base (Components|SkeletalMesh|GetAnimInstance (Variables|Character|GetMesh))))
  (Variables|/Game/Characters/Heroes/Mannequin/Animations/ABP_Mannequin_Base.ABP_Mannequin_Base_C|SetGameplayTag_IsADS _asabp_mannequin_base (Utilities|Enum|Equal(Enum) Speed "NewEnumerator1"))
  (bind _output_get (Variables|/Script/Engine.CharacterMovementComponent|SetMaxWalkSpeed (Variables|Character|GetCharacterMovement) (Utilities|Select :Index Speed :NewEnumerator0 0.0 :NewEnumerator1 1.5e+02 :NewEnumerator2 5e+02 :NewEnumerator3 7.5e+02)))
  (return _output_get))

(fn SetRemainingAmmo
  (params (newValue :type Integer))
  (switch Utilities|FlowControl|Switch|SwitchonEAmmoType (Variables|/Script/Octahedron.TP_WeaponComponent|GetAmmoType (Variables|Default|GetCurrentWeapon))
    (:None
      (return 0))
    (:Primary
      (return 999))
    (:Special
      (bind _output_get (Variables|Default|SetSpecialAmmoRemaining newValue))
      (return _output_get))
    (:Heavy
      (bind _output_get_2 (Variables|Default|SetHeavyAmmoRemaining newValue))
      (return _output_get_2))))

(fn SetWielderControlRotation
  (params (newRotator :type Rotator :default "0, 0, 0"))
  (Pawn|SetControlRotation (Pawn|GetController) newRotator)
  (return))

(fn TakeDamage
  (params (DamageInfo :type S%20Damage%20Info%20Structure) (Damage%20Causer :type Actor%20Object%20Reference) (Knockback%20Epicenter :type Vector :default "0, 0, 0"))
  (bind (_wasdamaged _wasdamagedtodeath _finaldamage _iscriticalhit) (Default|TakeDamage (Variables|Default|GetBPC_DamageSystem) DamageInfo Damage%20Causer Knockback%20Epicenter))
  (if _wasdamaged
    (bind _healthbar (Variables|Default|GetHealthBar)
      (:then
        (bind _maxhealth (CallFunction|GetMaxHealth))
        (bind _health (CallFunction|GetCurrentHealth))
        (bind _asw_dynamic_health_bar (Utilities|Casting|CastToW_DynamicHealthBar (UserInterface|GetWidget _healthbar))
          (:then
            (Default|UpdateValues _asw_dynamic_health_bar (/ _health _maxhealth)))
          (:CastFailed
            _)))
      (:else
        _)))
  (return _wasdamaged _wasdamagedtodeath _finaldamage _iscriticalhit))